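; Player leech character for a snake-style survival game, with a body of instanced static mesh cells built and detached in the construction script.
; While moving, the first cell snaps to the actor and the others lerp toward their predecessors' transforms.
; A Tick timer periodically removes a cell, and overlapping food adds one.
; Reaching the last cell triggers game over, disabling movement and showing the Level 2 fail screen.
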(event `self.ReceiveTick`
  (params (DeltaSeconds :type "Float (single-precision)"))
  (bind _instancedstaticmesh (`self.InstancedStaticMesh`))
  (bind _instancedstaticmesh_2 (`self.InstancedStaticMesh`))
  (bind _returnvalue (- (`InstancedStaticMeshComponent.GetInstanceCount` _instancedstaticmesh) 1))
  (bind _output_get (set `self.Second Counter` (+ DeltaSeconds (`self.Second Counter`))))
  (set `self.Game Score` (+ _output_get (`InstancedStaticMeshComponent.GetInstanceCount` (`self.InstancedStaticMesh`))))
  (if (>= (`self.Second Counter`) (`self.Countdown Amount`))
    (if (<= _returnvalue 0)
      (`InstancedStaticMeshComponent.AddInstance` _instancedstaticmesh_2 (`InstancedStaticMeshComponent.GetInstanceTransform` _instancedstaticmesh_2 (- (`InstancedStaticMeshComponent.GetInstanceCount` _instancedstaticmesh_2) 1) false) false)
      (bind _output_get_2 (set `self.Game Over` true))
      (if _output_get_2 :!label _label
        (`WidgetLayoutLibrary.RemoveAllWidgets`)
        (bind _returnvalue_2 (`|CreateWidget` "/Game/MyContent/New/BP/WB_EndScreenFail_Level2.WB_EndScreenFail_Level2_C"))
        (`UserWidget.AddToViewport` _returnvalue_2 0)
        (set `PlayerController.bShowMouseCursor` true (`GameplayStatics.GetPlayerController` 0))
        (`CharacterMovementComponent.DisableMovement` (`self.CharacterMovement`)))
      (else
        (`InstancedStaticMeshComponent.RemoveInstance` _instancedstaticmesh _returnvalue)
        (set `self.Second Counter` 0.0)
        (if (> (`KismetMathLibrary.VSize` (`self.GetVelocity`)) 10.0) :!label _label_2
          (`self.Lerp Locations`)
          (goto _label))))
    (else
      (goto _label_2))))

(event `Lerp Locations`
  (bind (_returnvalue_location _returnvalue_rotation) (`KismetMathLibrary.BreakTransform` (`self.GetTransform`)))
  (bind _instancedstaticmesh (`self.InstancedStaticMesh`))
  (bind (_output_location _output_rotation _output_scale) (`KismetMathLibrary.BreakTransform` (`|GetArrayItem` (`self.Cell Transform`))))
  (`KismetArrayLibrary.Array_Clear` (`self.Cell Transform`))
  (for _index (range (`InstancedStaticMeshComponent.GetInstanceCount` (`self.InstancedStaticMesh`)))
    (`KismetArrayLibrary.Array_Add` (`self.Cell Transform`) (`InstancedStaticMeshComponent.GetInstanceTransform` (`self.InstancedStaticMesh`) _index true)))
  (`InstancedStaticMeshComponent.UpdateInstanceTransform` (`self.InstancedStaticMesh`) 0 (`KismetMathLibrary.MakeTransform` _returnvalue_location _returnvalue_rotation _output_scale) true true false)
  (for (_array_element _array_index) (`self.Cell Transform`)
    (bind _returnvalue (+ _array_index 1))
    (bind (_returnvalue_location_2 _returnvalue_rotation_2 _returnvalue_scale) (`KismetMathLibrary.BreakTransform` (`KismetMathLibrary.TLerp` (`InstancedStaticMeshComponent.GetInstanceTransform` _instancedstaticmesh _returnvalue true) _array_element (`self.Cell Lerp Time`))))
    (`InstancedStaticMeshComponent.UpdateInstanceTransform` _instancedstaticmesh _returnvalue (`KismetMathLibrary.MakeTransform` _returnvalue_location_2 _returnvalue_rotation_2 _returnvalue_scale) true false false)))

(event `self.Sphere.OnComponentBeginOverlap`
  (params (OverlappedComponent :type "PrimitiveComponent Object Reference") (OtherActor :type "Actor Object Reference") (OtherComp :type "PrimitiveComponent Object Reference") (OtherBodyIndex :type Integer) (bFromSweep :type Boolean) (SweepResult :type "HitResult Structure (by ref)"))
  (bind _instancedstaticmesh (`self.InstancedStaticMesh`))
  (bind _yes_no (message `/Game/MyContent/New/BP/BPI_Food.Is Food` OtherActor))
  (if _yes_no
    (message `/Game/MyContent/New/BP/BPI_Food.Consume` OtherActor)
    (`InstancedStaticMeshComponent.AddInstance` _instancedstaticmesh (`InstancedStaticMeshComponent.GetInstanceTransform` _instancedstaticmesh (- (`InstancedStaticMeshComponent.GetInstanceCount` _instancedstaticmesh) 1) false) false)
    (`GameplayStatics.PlaySound2D` "/Game/MyContent/New/Audio/nomnombee.nomnombee" 1.0 1.0 0.0 null null)))

(fn `Is Food`
  (returns (`Yes/No` :type Boolean))
  (return false))

(fn `UserConstructionScript`
  (bind _instancedstaticmesh (`self.InstancedStaticMesh`))
  (`parent.UserConstructionScript`)
  (`SceneComponent.K2_DetachFromComponent` _instancedstaticmesh "KeepWorld" "KeepWorld" "KeepWorld" true)
  (`InstancedStaticMeshComponent.ClearInstances` _instancedstaticmesh)
  (for _index (range (+ (`self.Body Count`) 1))
    (`InstancedStaticMeshComponent.AddInstance` (`self.InstancedStaticMesh`) (`KismetMathLibrary.MakeTransform` (`KismetMathLibrary.MakeVector` (`KismetMathLibrary.Conv_IntToDouble` (+ (* _index (`self.Body Cell Spread`)) (`self.Offset`)))) (`KismetMathLibrary.MakeRotator` 90.0 0.0 140.0) (* (`self.Cell Scale`) (1.0 1.0 1.0))) false)))