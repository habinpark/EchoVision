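; BP_Food is a food pickup actor that spins in place until it is consumed.
; Construction gives it a random yaw, and BeginPlay picks a random spin speed that Tick applies each frame without delta-time scaling.
; IsFood always returns true to identify it as food, and Consume sets a short life span so the actor destroys itself shortly afterwards.
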(event `self.ReceiveBeginPlay`
  (set `self.Rotation speed` (* (`KismetMathLibrary.RandomFloat`) 0.7)))

(event `self.ReceiveTick`
  (params (DeltaSeconds :type "Float (single-precision)"))
  (`SceneComponent.K2_AddRelativeRotation` (`self.DefaultSceneRoot`) (`KismetMathLibrary.MakeRotator` 0.0 0.0 (`self.Rotation speed`)) false false))

(event `/Game/MyContent/New/BP/BPI_Food.Consume`
  (`self.SetLifeSpan` 0.1))

(fn `Is Food`
  (returns (`Yes/No` :type Boolean))
  (return true))

(fn `UserConstructionScript`
  (`SceneComponent.K2_AddRelativeRotation` (`self.DefaultSceneRoot`) (`KismetMathLibrary.MakeRotator` 0.0 0.0 (* (`KismetMathLibrary.RandomFloat`) 360.0)) false false))