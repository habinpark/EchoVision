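; BP_Leech is a leech whose segmented body of instanced mesh cells trails behind the actor as it moves.
; The construction script detaches the instanced mesh and rebuilds a line of evenly spaced, randomly rotated cells.
; While velocity is above a small threshold, Tick snapshots cell transforms, snaps the head cell to the actor and lerps each following cell toward its predecessor's previous transform.
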(event `self.ReceiveTick`
  (params (DeltaSeconds :type "Float (single-precision)"))
  (if (> (`KismetMathLibrary.VSize` (`self.GetVelocity`)) 10.0)
    (`self.Lerp Locations`)))

(event `Lerp Locations`
  (bind (_returnvalue_location _returnvalue_rotation) (`KismetMathLibrary.BreakTransform` (`self.GetTransform`)))
  (bind _instancedstaticmesh (`self.InstancedStaticMesh`))
  (bind (_output_location _output_rotation _output_scale) (`KismetMathLibrary.BreakTransform` (`|GetArrayItem` (`self.Cell Transform`))))
  (`KismetArrayLibrary.Array_Clear` (`self.Cell Transform`))
  (for _index (range (`InstancedStaticMeshComponent.GetInstanceCount` (`self.InstancedStaticMesh`)))
    (`KismetArrayLibrary.Array_Add` (`self.Cell Transform`) (`InstancedStaticMeshComponent.GetInstanceTransform` (`self.InstancedStaticMesh`) _index true)))
  (`InstancedStaticMeshComponent.UpdateInstanceTransform` (`self.InstancedStaticMesh`) 0 (`KismetMathLibrary.MakeTransform` _returnvalue_location _returnvalue_rotation _output_scale) true true false)
  (for (_array_element _array_index) (`self.Cell Transform`)
    (bind _returnvalue (+ _array_index 1))
    (`InstancedStaticMeshComponent.UpdateInstanceTransform` _instancedstaticmesh _returnvalue (`KismetMathLibrary.TLerp` (`InstancedStaticMeshComponent.GetInstanceTransform` _instancedstaticmesh _returnvalue true) _array_element (`self.Cell Lerp Time`)) true false false)))

(fn `UserConstructionScript`
  (bind _instancedstaticmesh (`self.InstancedStaticMesh`))
  (bind _returnvalue (* (`KismetMathLibrary.RandomFloat`) 360.0))
  (`parent.UserConstructionScript`)
  (`SceneComponent.K2_DetachFromComponent` _instancedstaticmesh "KeepWorld" "KeepWorld" "KeepWorld" true)
  (`InstancedStaticMeshComponent.ClearInstances` _instancedstaticmesh)
  (for _index (range (+ (`self.Body Count`) 1))
    (`InstancedStaticMeshComponent.AddInstance` (`self.InstancedStaticMesh`) (`KismetMathLibrary.MakeTransform` (`KismetMathLibrary.MakeVector` (`KismetMathLibrary.Conv_IntToDouble` (+ (* _index (`self.Body Cell Spread`)) (`self.Offset`)))) (`KismetMathLibrary.MakeRotator` _returnvalue _returnvalue _returnvalue) (* (`self.Cell Scale`) (1.0 1.0 1.0))) false)))